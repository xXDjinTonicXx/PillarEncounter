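; Player character for desktop play, driven by Enhanced Input with keyboard and mouse style move and look.
; The Desktop mapping context is added when the controller changes, feeding movement along actor forward and right and controller yaw with inverted pitch.
; Flashlight inputs find the level's BP_Flashlight by class lookup to toggle its light, or pick it up to a hold point and drop it.
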(event Input|EnhancedActionEvents|EnhancedInputActionIA_DesktopMove
  (params (ActionValue :type Vector%202D%20Structure) (ElapsedSeconds :type Float%20%28double-precision%29) (TriggeredSeconds :type Float%20%28double-precision%29) (InputAction :type Input%20Action%20Object%20Reference :default "/Game/Content/IA_DesktopMove.IA_DesktopMove"))
  (Pawn|Input|AddMovementInput (Transformation|GetActorForwardVector) (.y ActionValue) false)
  (Pawn|Input|AddMovementInput (Transformation|GetActorRightVector) (.x ActionValue) false))

(event Input|EnhancedActionEvents|EnhancedInputActionIA_DesktopLook
  (params (ActionValue :type Vector%202D%20Structure) (ElapsedSeconds :type Float%20%28double-precision%29) (TriggeredSeconds :type Float%20%28double-precision%29) (InputAction :type Input%20Action%20Object%20Reference :default "/Game/Content/IA_DesktopLook.IA_DesktopLook"))
  (Pawn|Input|AddControllerYawInput (.x ActionValue))
  (Pawn|Input|AddControllerPitchInput (* (.y ActionValue) -1.0)))

(event Input|EnhancedActionEvents|EnhancedInputActionIA_FlashlightToggle
  (params (ActionValue :type Boolean) (ElapsedSeconds :type Float%20%28double-precision%29) (TriggeredSeconds :type Float%20%28double-precision%29) (InputAction :type Input%20Action%20Object%20Reference :default "/Game/Content/IA_FlashlightToggle.IA_FlashlightToggle"))
  (bind _returnvalue (Actor|GetActorOfClass "/Game/Content/BP_Flashlight.BP_Flashlight_C"))
  (Class|FlashlightActor|ToggleLight _returnvalue))

(event Input|EnhancedActionEvents|EnhancedInputActionIA_FlashlightInteract
  (params (ActionValue :type Boolean) (ElapsedSeconds :type Float%20%28double-precision%29) (TriggeredSeconds :type Float%20%28double-precision%29) (InputAction :type Input%20Action%20Object%20Reference :default "/Game/Content/IA_FlashlightInteract.IA_FlashlightInteract"))
  (:Started
    (bind _returnvalue (Actor|GetActorOfClass "/Game/Content/BP_Flashlight.BP_Flashlight_C"))
    (if (Class|FlashlightActor|IsHeld _returnvalue)
      (Class|FlashlightActor|Drop _returnvalue)
      (else
        (Class|FlashlightActor|PickUp _returnvalue (Variables|Default|GetFlashlightHoldPoint))))))

(event EventBeginPlay)

(event EventControllerChanged
  (params (OldController :type Controller%20Object%20Reference) (NewController :type Controller%20Object%20Reference))
  (Input|AddMappingContext (PlayerController|LocalPlayerSubsystems|GetEnhancedInputLocalPlayerSubsystem (Game|GetPlayerController 0)) "/Game/Content/IMC_Desktop.IMC_Desktop" 0 "(bIgnoreAllPressedKeysUntilRelease=True,bForceImmediately=False,bNotifyUserSettings=False)"))

(fn ConstructionScript)