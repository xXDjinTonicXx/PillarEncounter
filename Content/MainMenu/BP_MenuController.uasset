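; BP_MenuController is the main menu player controller, which chooses between joining a host and showing the menu on BeginPlay.
; With a head-mounted display enabled, it waits briefly and runs an "open" console command built from HostIP, skipping the menu.
; Otherwise it creates WBP_Mainmenu, adds it to the viewport, shows the mouse cursor and switches to UI-only input focused on that widget.
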(event EventBeginPlay
  (if (Class|HeadMountedDisplayFunctionLibrary|IsHeadMountedDisplayEnabled)
    (Utilities|FlowControl|Delay 0.2)
    (Development|ExecuteConsoleCommand (Utilities|String|Append "open " (Variables|Default|GetHostIP)) 0)
    (else
      (bind _returnvalue (UserInterface|CreateWidget "/Game/MainMenu/WBP_Mainmenu.WBP_Mainmenu_C" self))
      (UserInterface|Viewport|AddtoViewport _returnvalue 0)
      (Variables|Default|SetbShowMouseCursor true)
      (Input|SetInputModeUIOnly self _returnvalue "DoNotLock" false))))

(event EventTick
  (params (DeltaSeconds :type Float%20%28single-precision%29)))

(fn ConstructionScript)